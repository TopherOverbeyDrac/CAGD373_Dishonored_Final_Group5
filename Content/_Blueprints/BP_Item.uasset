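; BP_Item is a world pickup actor whose mesh is set in the construction script from its ItemData.
; On interaction it passes ItemData to the interacting player's PickUpItem.
; A timeline then lerps the item from its current location toward the player's live position, and the actor destroys itself when the timeline finishes.
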(event `/Game/_Blueprints/_Interfaces/BPI_Interactable.OnInteract`
  (params (InteractingPlayer :type "/Game/Original_Level_Stuff/FirstPerson/Blueprints/BP_FirstPersonCharacter Object Reference"))
  (`/Game/Original_Level_Stuff/FirstPerson/Blueprints/BP_FirstPersonCharacter.PickUpItem` InteractingPlayer (`self.ItemData`))
  (bind (_direction _movetime) (`Timeline|Timeline`)
    (:`Update`
      (`self.K2_SetActorLocation` (`KismetMathLibrary.VLerp` (`self.K2_GetActorLocation`) (`self.K2_GetActorLocation` InteractingPlayer) _movetime)))
    (:`Finished`
      (`self.K2_DestroyActor`))))

(fn `UserConstructionScript`
  (`StaticMeshComponent.SetStaticMesh` (`self.StaticMesh`) (`/Game/_Blueprints/_Data/PD_Item.StaticMesh` (`self.ItemData`))))