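; BP_Item is an interactable pickup whose mesh and sound come from its ItemData in the Construction Script, with RandomSound as fallback.
; On interact, it passes ItemData to the player's PickUpItem, plays the sound, then lerps toward the player on a Timeline and destroys itself.
; If the player is holding whale oil, interacting only clears that flag and skips the pickup.
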(event `/Game/_Blueprints/_Interfaces/BPI_Interactable.OnInteract`
  (params (InteractingPlayer :type "/Game/Original_Level_Stuff/FirstPerson/Blueprints/BP_FirstPersonCharacter Object Reference"))
  (bind _sound (`self.Sound`))
  (if (`/Game/Original_Level_Stuff/FirstPerson/Blueprints/BP_FirstPersonCharacter.IsHoldingWhaleOil` InteractingPlayer)
    (set `/Game/Original_Level_Stuff/FirstPerson/Blueprints/BP_FirstPersonCharacter.IsHoldingWhaleOil` false InteractingPlayer)
    (else
      (`/Game/Original_Level_Stuff/FirstPerson/Blueprints/BP_FirstPersonCharacter.PickUpItem` InteractingPlayer (`self.ItemData`))
      (`/Engine/EditorBlueprintResources/StandardMacros.IsValid` _sound
        (:`Is Valid`
          (`AudioComponent.Play` _sound 0.0)
          (bind (_direction _movetime) (`Timeline|Timeline`)
            (:`Update`
              (`self.K2_SetActorLocation` (`KismetMathLibrary.VLerp` (`self.K2_GetActorLocation`) (`self.K2_GetActorLocation` InteractingPlayer) _movetime)))
            (:`Finished`
              (`self.K2_DestroyActor`))))))))

(fn `UserConstructionScript`
  (bind _itemdata (`self.ItemData`))
  (bind _randomsound (`/Game/_Blueprints/_Data/PD_Item.RandomSound` _itemdata))
  (bind _sound (`/Game/_Blueprints/_Data/PD_Item.Sound` _itemdata))
  (`StaticMeshComponent.SetStaticMesh` (`self.StaticMesh`) (`/Game/_Blueprints/_Data/PD_Item.StaticMesh` _itemdata))
  (`/Engine/EditorBlueprintResources/StandardMacros.IsValid` _sound
    (:`Is Valid`
      (`AudioComponent.SetSound` (`self.Sound`) _sound))
    (:`Is Not Valid`
      (`/Engine/EditorBlueprintResources/StandardMacros.IsValid` _randomsound
        (:`Is Valid`
          (`AudioComponent.SetSound` (`self.Sound`) _randomsound))))))