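; Wall of Light security gate, powered by a whale oil tank, that electrocutes actors crossing it.
; Interacting while holding a tank snaps it into the receptacle and starts idle lightning beams between four coils; removing it shuts them off.
; While powered, an overlap flashes kill beams at the velocity-predicted target position and notifies BPI_Killable actors.
; An outer audio collider plays an alarm for Person-tagged actors, then a friend-detected sound on exit.
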(event `self.ReceiveBeginPlay`
  (bind _coil1 (`self.Coil1`))
  (bind _coil2 (`self.Coil2`))
  (bind _coil3 (`self.Coil3`))
  (bind _coil4 (`self.Coil4`))
  (bind _lightning5 (`self.Lightning5`))
  (bind _lightning6 (`self.Lightning6`))
  (bind _coil1_2 (`self.Coil1`))
  (bind _coil2_2 (`self.Coil2`))
  (bind _coil3_2 (`self.Coil3`))
  (bind _coil4_2 (`self.Coil4`))
  (bind _lightning1 (`self.Lightning1`))
  (bind _lightning2 (`self.Lightning2`))
  (bind _lightning3 (`self.Lightning3`))
  (bind _lightning4 (`self.Lightning4`))
  (bind _returnvalue_location (`KismetMathLibrary.BreakTransform` (`SceneComponent.GetSocketTransform` _coil2_2 "PylonLower" "RTS_World")))
  (bind (_returnvalue_location_2 _returnvalue_rotation _returnvalue_scale) (`KismetMathLibrary.BreakTransform` (`SceneComponent.GetSocketTransform` _coil3_2 "PylonUpper" "RTS_World")))
  (bind _returnvalue_location_3 (`KismetMathLibrary.BreakTransform` (`SceneComponent.GetSocketTransform` _coil3_2 "PylonLower" "RTS_World")))
  (bind (_returnvalue_location_4 _returnvalue_rotation_2 _returnvalue_scale_2) (`KismetMathLibrary.BreakTransform` (`SceneComponent.GetSocketTransform` _coil4_2 "PylonUpper" "RTS_World")))
  (bind _returnvalue_location_5 (`KismetMathLibrary.BreakTransform` (`SceneComponent.GetSocketTransform` _coil4_2 "PylonLower" "RTS_World")))
  (bind (_returnvalue_location_6 _returnvalue_rotation_3 _returnvalue_scale_3) (`KismetMathLibrary.BreakTransform` (`SceneComponent.GetSocketTransform` (`self.Coil4`) "PylonUpper" "RTS_World")))
  (bind (_returnvalue_location_7 _returnvalue_rotation_4 _returnvalue_scale_4) (`KismetMathLibrary.BreakTransform` (`SceneComponent.GetSocketTransform` _coil1 "PylonUpper" "RTS_World")))
  (bind (_returnvalue_location_8 _returnvalue_rotation_5 _returnvalue_scale_5) (`KismetMathLibrary.BreakTransform` (`SceneComponent.GetSocketTransform` _coil2 "PylonUpper" "RTS_World")))
  (bind _returnvalue_location_9 (`KismetMathLibrary.BreakTransform` (`SceneComponent.GetSocketTransform` _coil2 "PylonLower" "RTS_World")))
  (bind (_returnvalue_location_10 _returnvalue_rotation_6 _returnvalue_scale_6) (`KismetMathLibrary.BreakTransform` (`SceneComponent.GetSocketTransform` _coil3 "PylonUpper" "RTS_World")))
  (bind _returnvalue_location_11 (`KismetMathLibrary.BreakTransform` (`SceneComponent.GetSocketTransform` _coil3 "PylonLower" "RTS_World")))
  (bind (_returnvalue_location_12 _returnvalue_rotation_7 _returnvalue_scale_7) (`KismetMathLibrary.BreakTransform` (`SceneComponent.GetSocketTransform` _coil4 "PylonUpper" "RTS_World")))
  (bind _returnvalue_location_13 (`KismetMathLibrary.BreakTransform` (`SceneComponent.GetSocketTransform` _coil4 "PylonLower" "RTS_World")))
  (bind _returnvalue_location_14 (`KismetMathLibrary.BreakTransform` (`SceneComponent.GetSocketTransform` _coil1 "PylonLower" "RTS_World")))
  (bind (_returnvalue_location_15 _returnvalue_rotation_8 _returnvalue_scale_8) (`KismetMathLibrary.BreakTransform` (`SceneComponent.GetSocketTransform` (`self.Coil3`) "PylonUpper" "RTS_World")))
  (bind _returnvalue_location_16 (`KismetMathLibrary.BreakTransform` (`SceneComponent.GetSocketTransform` (`self.Coil1`) "PylonLower" "RTS_World")))
  (bind _returnvalue_location_17 (`KismetMathLibrary.BreakTransform` (`SceneComponent.GetSocketTransform` (`self.Coil2`) "PylonLower" "RTS_World")))
  (bind (_returnvalue_location_18 _returnvalue_rotation_9 _returnvalue_scale_9) (`KismetMathLibrary.BreakTransform` (`SceneComponent.GetSocketTransform` _coil1_2 "PylonUpper" "RTS_World")))
  (bind _returnvalue_location_19 (`KismetMathLibrary.BreakTransform` (`SceneComponent.GetSocketTransform` _coil1_2 "PylonLower" "RTS_World")))
  (bind (_returnvalue_location_20 _returnvalue_rotation_10 _returnvalue_scale_10) (`KismetMathLibrary.BreakTransform` (`SceneComponent.GetSocketTransform` _coil2_2 "PylonUpper" "RTS_World")))
  (`|ExecutionSequence`
    (:`then_0`
      (`NiagaraFunctionLibrary.SpawnSystemAtLocation` null _returnvalue_location_7 _returnvalue_rotation_4 _returnvalue_scale_4)
      (`NiagaraComponent.SetVariablePosition` (`self.LightningKill1`) "BeamStart" _returnvalue_location_7)
      (`NiagaraComponent.SetVariablePosition` (`self.LightningKill2`) "BeamStart" _returnvalue_location_14)
      (`NiagaraComponent.SetVariablePosition` (`self.LightningKill1`) "BeamEnd" _returnvalue_location_7)
      (`NiagaraComponent.SetVariablePosition` (`self.LightningKill2`) "BeamEnd" _returnvalue_location_14)
      (`NiagaraFunctionLibrary.SpawnSystemAtLocation` null _returnvalue_location_8 _returnvalue_rotation_5 _returnvalue_scale_5)
      (`NiagaraComponent.SetVariablePosition` (`self.LightningKill3`) "BeamStart" _returnvalue_location_8)
      (`NiagaraComponent.SetVariablePosition` (`self.LightningKill4`) "BeamStart" _returnvalue_location_9)
      (`NiagaraComponent.SetVariablePosition` (`self.LightningKill3`) "BeamEnd" _returnvalue_location_8)
      (`NiagaraComponent.SetVariablePosition` (`self.LightningKill4`) "BeamEnd" _returnvalue_location_9)
      (`NiagaraFunctionLibrary.SpawnSystemAtLocation` null _returnvalue_location_10 _returnvalue_rotation_6 _returnvalue_scale_6)
      (`NiagaraComponent.SetVariablePosition` (`self.LightningKill5`) "BeamStart" _returnvalue_location_10)
      (`NiagaraComponent.SetVariablePosition` (`self.LightningKill6`) "BeamStart" _returnvalue_location_11)
      (`NiagaraComponent.SetVariablePosition` (`self.LightningKill5`) "BeamEnd" _returnvalue_location_10)
      (`NiagaraComponent.SetVariablePosition` (`self.LightningKill6`) "BeamEnd" _returnvalue_location_11)
      (`NiagaraFunctionLibrary.SpawnSystemAtLocation` null _returnvalue_location_12 _returnvalue_rotation_7 _returnvalue_scale_7)
      (`NiagaraComponent.SetVariablePosition` (`self.LightningKill7`) "BeamStart" _returnvalue_location_12)
      (`NiagaraComponent.SetVariablePosition` (`self.LightningKill8`) "BeamStart" _returnvalue_location_13)
      (`NiagaraComponent.SetVariablePosition` (`self.LightningKill7`) "BeamEnd" _returnvalue_location_12)
      (`NiagaraComponent.SetVariablePosition` (`self.LightningKill8`) "BeamEnd" _returnvalue_location_13)
      (`ActorComponent.Deactivate` (`self.LightningKill1`))
      (`ActorComponent.Deactivate` (`self.LightningKill2`))
      (`ActorComponent.Deactivate` (`self.LightningKill3`))
      (`ActorComponent.Deactivate` (`self.LightningKill4`))
      (`ActorComponent.Deactivate` (`self.LightningKill5`))
      (`ActorComponent.Deactivate` (`self.LightningKill6`))
      (`ActorComponent.Deactivate` (`self.LightningKill7`))
      (`ActorComponent.Deactivate` (`self.LightningKill8`)))
    (:`then_1`
      (`NiagaraFunctionLibrary.SpawnSystemAtLocation` null _returnvalue_location_18 _returnvalue_rotation_9 _returnvalue_scale_9)
      (`NiagaraComponent.SetVariablePosition` _lightning1 "BeamStart" _returnvalue_location_18)
      (`NiagaraComponent.SetVariablePosition` _lightning1 "BeamEnd" _returnvalue_location_19)
      (`NiagaraFunctionLibrary.SpawnSystemAtLocation` null _returnvalue_location_20 _returnvalue_rotation_10 _returnvalue_scale_10)
      (`NiagaraComponent.SetVariablePosition` _lightning2 "BeamStart" _returnvalue_location_20)
      (`NiagaraComponent.SetVariablePosition` _lightning2 "BeamEnd" _returnvalue_location)
      (`NiagaraFunctionLibrary.SpawnSystemAtLocation` null _returnvalue_location_2 _returnvalue_rotation _returnvalue_scale)
      (`NiagaraComponent.SetVariablePosition` _lightning3 "BeamStart" _returnvalue_location_2)
      (`NiagaraComponent.SetVariablePosition` _lightning3 "BeamEnd" _returnvalue_location_3)
      (`NiagaraFunctionLibrary.SpawnSystemAtLocation` null _returnvalue_location_4 _returnvalue_rotation_2 _returnvalue_scale_2)
      (`NiagaraComponent.SetVariablePosition` _lightning4 "BeamStart" _returnvalue_location_4)
      (`NiagaraComponent.SetVariablePosition` _lightning4 "BeamEnd" _returnvalue_location_5)
      (`NiagaraFunctionLibrary.SpawnSystemAtLocation` null _returnvalue_location_15 _returnvalue_rotation_8 _returnvalue_scale_8)
      (`NiagaraComponent.SetVariablePosition` _lightning5 "BeamStart" _returnvalue_location_15)
      (`NiagaraComponent.SetVariablePosition` _lightning5 "BeamEnd" _returnvalue_location_16)
      (`NiagaraFunctionLibrary.SpawnSystemAtLocation` null _returnvalue_location_6 _returnvalue_rotation_3 _returnvalue_scale_3)
      (`NiagaraComponent.SetVariablePosition` _lightning6 "BeamStart" _returnvalue_location_6)
      (`NiagaraComponent.SetVariablePosition` _lightning6 "BeamEnd" _returnvalue_location_17))))

(event `self.KillCollider.OnComponentBeginOverlap`
  (params (OverlappedComponent :type "PrimitiveComponent Object Reference") (OtherActor :type "Actor Object Reference") (OtherComp :type "PrimitiveComponent Object Reference") (OtherBodyIndex :type Integer) (bFromSweep :type Boolean) (SweepResult :type "HitResult Structure (by ref)"))
  (bind _targetlocation (`self.TargetLocation`))
  (bind _targetlocation_2 (`self.TargetLocation`))
  (bind _targetlocation_3 (`self.TargetLocation`))
  (bind _targetlocation_4 (`self.TargetLocation`))
  (bind _other_actor (`self.Other Actor`))
  (bind _other_actor_2 (`self.Other Actor`))
  (bind (_returnvalue_x _returnvalue_y) (`KismetMathLibrary.BreakVector` (`self.GetVelocity` _other_actor_2)))
  (bind (_returnvalue_x_2 _returnvalue_y_2 _returnvalue_z) (`KismetMathLibrary.BreakVector` (`self.K2_GetActorLocation` _other_actor_2)))
  (if (`self.IsTankInReceptacle`)
    (set `self.Other Actor` OtherActor)
    (`/Engine/EditorBlueprintResources/StandardMacros.IsValid` (`self.Other Actor`)
      (:`Is Valid`
        (`|ExecutionSequence`
          (:`then_0`
            (`GameplayStatics.PlaySoundAtLocation` "/Game/_Audio/SW_Electricity_zap.SW_Electricity_zap" (`self.K2_GetActorLocation`) (struct) 1.0 1.0 0.0 null null null null))
          (:`then_1`
            (set `self.TargetLocation` (`KismetMathLibrary.MakeVector` (+ (* _returnvalue_x (`self.VelocityModifier`)) _returnvalue_x_2) (+ (* _returnvalue_y (`self.VelocityModifier`)) _returnvalue_y_2) _returnvalue_z))
            (`NiagaraComponent.SetVariablePosition` (`self.LightningKill1`) "BeamEnd" _targetlocation_2)
            (`NiagaraComponent.SetVariablePosition` (`self.LightningKill2`) "BeamEnd" _targetlocation_2)
            (`NiagaraComponent.SetVariablePosition` (`self.LightningKill3`) "BeamEnd" _targetlocation_3)
            (`NiagaraComponent.SetVariablePosition` (`self.LightningKill4`) "BeamEnd" _targetlocation_3)
            (`NiagaraComponent.SetVariablePosition` (`self.LightningKill5`) "BeamEnd" _targetlocation_4)
            (`NiagaraComponent.SetVariablePosition` (`self.LightningKill6`) "BeamEnd" _targetlocation_4)
            (`NiagaraComponent.SetVariablePosition` (`self.LightningKill7`) "BeamEnd" _targetlocation)
            (`NiagaraComponent.SetVariablePosition` (`self.LightningKill8`) "BeamEnd" _targetlocation)
            (`ActorComponent.Deactivate` (`self.Lightning1`))
            (`ActorComponent.Deactivate` (`self.Lightning2`))
            (`ActorComponent.Deactivate` (`self.Lightning3`))
            (`ActorComponent.Deactivate` (`self.Lightning4`))
            (`ActorComponent.Deactivate` (`self.Lightning5`))
            (`ActorComponent.Deactivate` (`self.Lightning6`))
            (`ActorComponent.Activate` (`self.LightningKill1`) true)
            (`ActorComponent.Activate` (`self.LightningKill2`) true)
            (`ActorComponent.Activate` (`self.LightningKill3`) true)
            (`ActorComponent.Activate` (`self.LightningKill4`) true)
            (`ActorComponent.Activate` (`self.LightningKill5`) true)
            (`ActorComponent.Activate` (`self.LightningKill6`) true)
            (`ActorComponent.Activate` (`self.LightningKill7`) true)
            (`ActorComponent.Activate` (`self.LightningKill8`) true)
            (`KismetSystemLibrary.Delay` 0.1)
            (`ActorComponent.Deactivate` (`self.LightningKill1`))
            (`ActorComponent.Deactivate` (`self.LightningKill2`))
            (`ActorComponent.Deactivate` (`self.LightningKill3`))
            (`ActorComponent.Deactivate` (`self.LightningKill4`))
            (`ActorComponent.Deactivate` (`self.LightningKill5`))
            (`ActorComponent.Deactivate` (`self.LightningKill6`))
            (`ActorComponent.Deactivate` (`self.LightningKill7`))
            (`ActorComponent.Deactivate` (`self.LightningKill8`))
            (`ActorComponent.Activate` (`self.Lightning1`) false)
            (`ActorComponent.Activate` (`self.Lightning2`) false)
            (`ActorComponent.Activate` (`self.Lightning3`) false)
            (`ActorComponent.Activate` (`self.Lightning4`) false)
            (`ActorComponent.Activate` (`self.Lightning5`) false)
            (`ActorComponent.Activate` (`self.Lightning6`) false))
          (:`then_2`
            (if (`KismetSystemLibrary.DoesImplementInterface` _other_actor "/Game/_Blueprints/_Interfaces/BPI_Killable.BPI_Killable_C")
              (message `/Game/_Blueprints/_Interfaces/BPI_Killable.OnKilled` _other_actor self))))))))

(event `self.AudioCollider.OnComponentBeginOverlap`
  (params (OverlappedComponent :type "PrimitiveComponent Object Reference") (OtherActor :type "Actor Object Reference") (OtherComp :type "PrimitiveComponent Object Reference") (OtherBodyIndex :type Integer) (bFromSweep :type Boolean) (SweepResult :type "HitResult Structure (by ref)"))
  (if (`self.IsTankInReceptacle`)
    (if (`self.ActorHasTag` OtherActor "Person")
      (`AudioComponent.Play` (`self.EnemyAlarm`) 0.0))))

(event `self.AudioCollider.OnComponentEndOverlap`
  (params (OverlappedComponent :type "PrimitiveComponent Object Reference") (OtherActor :type "Actor Object Reference") (OtherComp :type "PrimitiveComponent Object Reference") (OtherBodyIndex :type Integer))
  (if (`self.IsTankInReceptacle`)
    (if (`self.ActorHasTag` OtherActor "Person")
      (`AudioComponent.Stop` (`self.EnemyAlarm`))
      (`GameplayStatics.PlaySoundAtLocation` "/Game/_Audio/SW_Friend_detected.SW_Friend_detected" (`self.K2_GetActorLocation`) (struct) 1.0 1.0 0.0 null null null null))))

(event `/Game/_Blueprints/_Interfaces/BPI_Interactable.OnInteract`
  (params (InteractingPlayer :type "/Game/Original_Level_Stuff/FirstPerson/Blueprints/BP_FirstPersonCharacter Object Reference"))
  (bind _whaleoilref (`/Game/Original_Level_Stuff/FirstPerson/Blueprints/BP_FirstPersonCharacter.WhaleOilRef` InteractingPlayer))
  (if (`/Game/Original_Level_Stuff/FirstPerson/Blueprints/BP_FirstPersonCharacter.IsHoldingWhaleOil` InteractingPlayer)
    (`/Engine/EditorBlueprintResources/StandardMacros.IsValid` _whaleoilref
      (:`Is Valid`
        (`PrimitiveComponent.SetSimulatePhysics` (`/Game/_Blueprints/Interactables/BP_WhaleOilTank.TankMesh` _whaleoilref) false)
        (`self.K2_AttachToComponent` _whaleoilref (`self.TankLocation`) "None" "SnapToTarget" "SnapToTarget" "KeepRelative" false)
        (`PrimitiveComponent.SetCollisionEnabled` (`/Game/_Blueprints/Interactables/BP_WhaleOilTank.TankMesh` _whaleoilref) "QueryAndPhysics")
        (set `self.IsTankInReceptacle` true)
        (set `/Game/Original_Level_Stuff/FirstPerson/Blueprints/BP_FirstPersonCharacter.IsHoldingWhaleOil` false InteractingPlayer)
        (`ActorComponent.Activate` (`self.Lightning1`) false)
        (`ActorComponent.Activate` (`self.Lightning2`) false)
        (`ActorComponent.Activate` (`self.Lightning3`) false)
        (`ActorComponent.Activate` (`self.Lightning4`) false)
        (`ActorComponent.Activate` (`self.Lightning5`) false)
        (`ActorComponent.Activate` (`self.Lightning6`) false)
        (`AudioComponent.Play` (`self.Static`) 0.0)))))

(event `self.TankChecker.OnComponentEndOverlap`
  (params (OverlappedComponent :type "PrimitiveComponent Object Reference") (OtherActor :type "Actor Object Reference") (OtherComp :type "PrimitiveComponent Object Reference") (OtherBodyIndex :type Integer))
  (if (`KismetSystemLibrary.DoesImplementInterface` OtherActor "/Game/_Blueprints/_Interfaces/BPI_Interactable.BPI_Interactable_C")
    (set `self.IsTankInReceptacle` false)
    (`ActorComponent.Deactivate` (`self.Lightning1`))
    (`ActorComponent.Deactivate` (`self.Lightning2`))
    (`ActorComponent.Deactivate` (`self.Lightning3`))
    (`ActorComponent.Deactivate` (`self.Lightning4`))
    (`ActorComponent.Deactivate` (`self.Lightning5`))
    (`ActorComponent.Deactivate` (`self.Lightning6`))
    (`AudioComponent.Stop` (`self.Static`))))

(fn `UserConstructionScript`)