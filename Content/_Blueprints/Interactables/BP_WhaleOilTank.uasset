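; BP_WhaleOilTank is an explosive interactable tank that the player can carry and throw.
; Interact attaches it to the player's hold point; throw restores physics and applies a camera-forward impulse.
; A thrown tank's first hit, or being killed while unthrown, triggers a delayed explosion, whereas being killed after throwing only fizzles.
; The blast briefly enables overlap collision, killing BPI_Killable actors and knocking back first-person characters.
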(event `/Game/_Blueprints/_Interfaces/BPI_Interactable.OnInteract`
  (params (InteractingPlayer :type "/Game/Original_Level_Stuff/FirstPerson/Blueprints/BP_FirstPersonCharacter Object Reference"))
  (`/Engine/EditorBlueprintResources/StandardMacros.IsValid` InteractingPlayer
    (:`Is Valid`
      (if (not (`/Game/Original_Level_Stuff/FirstPerson/Blueprints/BP_FirstPersonCharacter.IsHoldingWhaleOil` InteractingPlayer))
        (`PrimitiveComponent.SetSimulatePhysics` (`self.TankMesh`) false)
        (`PrimitiveComponent.SetCollisionEnabled` (`self.TankMesh`) "NoCollision")
        (`PrimitiveComponent.SetPhysicsLinearVelocity` (`self.TankMesh`) (0.0 0.0 0.0) false "None")
        (`PrimitiveComponent.SetPhysicsAngularVelocityInDegrees` (`self.TankMesh`) (0.0 0.0 0.0) false "None")
        (`self.K2_AttachToComponent` (`/Game/Original_Level_Stuff/FirstPerson/Blueprints/BP_FirstPersonCharacter.HoldLocation` InteractingPlayer) "None" "SnapToTarget" "SnapToTarget" "KeepRelative" false)
        (set `/Game/Original_Level_Stuff/FirstPerson/Blueprints/BP_FirstPersonCharacter.IsHoldingWhaleOil` true InteractingPlayer)))))

(event `/Game/_Blueprints/_Interfaces/BPI_Throwable.OnThrow`
  (params (ThrowingPlayer :type "/Game/Original_Level_Stuff/FirstPerson/Blueprints/BP_FirstPersonCharacter Object Reference"))
  (if (`/Game/Original_Level_Stuff/FirstPerson/Blueprints/BP_FirstPersonCharacter.IsHoldingWhaleOil` ThrowingPlayer)
    (`PrimitiveComponent.SetSimulatePhysics` (`self.TankMesh`) true)
    (`PrimitiveComponent.SetCollisionEnabled` (`self.TankMesh`) "QueryAndPhysics")
    (`SceneComponent.K2_DetachFromComponent` (`self.TankMesh`) "KeepWorld" "KeepWorld" "KeepRelative" true)
    (`PrimitiveComponent.AddImpulse` (`self.TankMesh`) (* (`SceneComponent.GetForwardVector` (`/Game/Original_Level_Stuff/FirstPerson/Blueprints/BP_FirstPersonCharacter.FirstPersonCamera` ThrowingPlayer)) (`self.ThrowStrength`)) "None" false)
    (set `/Game/Original_Level_Stuff/FirstPerson/Blueprints/BP_FirstPersonCharacter.IsHoldingWhaleOil` false ThrowingPlayer)
    (set `self.IsThrown` true)))

(event `self.TankMesh.OnComponentHit`
  (params (HitComponent :type "PrimitiveComponent Object Reference") (OtherActor :type "Actor Object Reference") (OtherComp :type "PrimitiveComponent Object Reference") (NormalImpulse :type "Vector Structure") (Hit :type "HitResult Structure (by ref)"))
  (if (`self.IsThrown`)
    (`/Engine/EditorBlueprintResources/StandardMacros.DoOnce` false
      (:`Completed`
        (`GameplayStatics.PlaySoundAtLocation` "/Game/_Audio/SW_GlassCrack.SW_GlassCrack" (`self.K2_GetActorLocation`) (struct) 1.0 1.0 0.0 null null null null)
        (`KismetSystemLibrary.Delay` 0.75)
        (`NiagaraFunctionLibrary.SpawnSystemAtLocation` "/Game/_VFX/NS_Explosion.NS_Explosion" (`SceneComponent.RelativeLocation` (`self.TankMesh`)))
        (`GameplayStatics.PlaySoundAtLocation` "/Game/_Audio/SC_RandomExplosion.SC_RandomExplosion" (`self.K2_GetActorLocation`) (struct) 1.0 1.0 0.0 null null null null)
        (`PrimitiveComponent.SetCollisionEnabled` (`self.ExplosionCollision`) "QueryOnly")
        (`KismetSystemLibrary.DelayUntilNextFrame`)
        (`self.K2_DestroyActor`)))))

(event `self.ReceiveActorBeginOverlap`
  (params (OtherActor :type "Actor Object Reference"))
  (if (`KismetSystemLibrary.DoesImplementInterface` OtherActor "/Game/_Blueprints/_Interfaces/BPI_Killable.BPI_Killable_C")
    (bind _asbp_first_person_character (cast `/Game/Original_Level_Stuff/FirstPerson/Blueprints/BP_FirstPersonCharacter` OtherActor)
      (:`then`
        (`/Engine/EditorBlueprintResources/StandardMacros.IsValid` _asbp_first_person_character
          (:`Is Valid`
            (message `/Game/_Blueprints/_Interfaces/BPI_Killable.OnKilled` OtherActor self)
            (bind (_returnvalue_x _returnvalue_y) (`KismetMathLibrary.BreakVector` (* (`KismetMathLibrary.Normal` (- (`self.K2_GetActorLocation` _asbp_first_person_character) (`self.K2_GetActorLocation`))) (`self.ExplosionStrength`))))
            (`PrimitiveComponent.AddImpulse` (`Character.Mesh` _asbp_first_person_character) (`KismetMathLibrary.MakeVector` _returnvalue_x _returnvalue_y) "None" false))))
      (:`CastFailed`
        (message `/Game/_Blueprints/_Interfaces/BPI_Killable.OnKilled` OtherActor self)))))

(event `/Game/_Blueprints/_Interfaces/BPI_Killable.OnKilled`
  (params (DamageCauser :type "Actor Object Reference"))
  (if (`self.IsThrown`)
    (`NiagaraFunctionLibrary.SpawnSystemAtLocation` "/Game/_VFX/NS_Fizzle.NS_Fizzle" (`SceneComponent.RelativeLocation` (`self.TankMesh`)))
    (`self.K2_DestroyActor`)
    (else
      (`KismetSystemLibrary.Delay` 0.75)
      (`GameplayStatics.PlaySoundAtLocation` "/Game/_Audio/SC_RandomExplosion.SC_RandomExplosion" (`self.K2_GetActorLocation`) (struct) 1.0 1.0 0.0 null null null null)
      (`NiagaraFunctionLibrary.SpawnSystemAtLocation` "/Game/_VFX/NS_Explosion.NS_Explosion" (`SceneComponent.RelativeLocation` (`self.TankMesh`)))
      (`PrimitiveComponent.SetCollisionEnabled` (`self.ExplosionCollision`) "QueryOnly")
      (`KismetSystemLibrary.DelayUntilNextFrame`)
      (`self.K2_DestroyActor`))))

(fn `UserConstructionScript`)