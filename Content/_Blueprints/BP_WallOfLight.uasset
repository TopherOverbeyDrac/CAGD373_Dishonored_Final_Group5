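; BP_WallOfLight is a hazard actor that knocks out the first-person player on overlap and sends them back to the level's PlayerStart.
; On overlap it disables input and capsule collision and turns the character mesh into a physics ragdoll for a few seconds.
; It then restores collision, reattaches the mesh to the capsule at its default offset, teleports the character to the cached PlayerStart transform and re-enables input.
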(event `self.ReceiveBeginPlay`
  (bind _returnvalue (`GameplayStatics.GetActorOfClass` "/Script/Engine.PlayerStart"))
  (set `self.PlayerStart` _returnvalue))

(event `self.ReceiveActorBeginOverlap`
  (params (OtherActor :type "Actor Object Reference"))
  (bind _playerstart (`self.PlayerStart`))
  (bind (_returnvalue_x _returnvalue_y _returnvalue_z) (`KismetMathLibrary.BreakVector` (`self.K2_GetActorLocation` _playerstart)))
  (bind _mesh (`Character.Mesh` (`self.FirstPersonCharacter`)))
  (bind _mesh_2 (`Character.Mesh` (`self.FirstPersonCharacter`)))
  (bind _mesh_3 (`Character.Mesh` (`self.FirstPersonCharacter`)))
  (bind _asbp_first_person_character (cast `/Game/Original_Level_Stuff/FirstPerson/Blueprints/BP_FirstPersonCharacter` OtherActor))
  (bind _output_get (set `self.FirstPersonCharacter` _asbp_first_person_character))
  (`/Engine/EditorBlueprintResources/StandardMacros.IsValid` _output_get
    (:`Is Valid`
      (`self.DisableInput` (`self.FirstPersonCharacter`) (`GameplayStatics.GetPlayerController` 0))
      (`PrimitiveComponent.SetCollisionEnabled` (`Character.CapsuleComponent` (`self.FirstPersonCharacter`)) "NoCollision")
      (`PrimitiveComponent.SetCollisionObjectType` _mesh_2 "ECC_PhysicsBody")
      (`PrimitiveComponent.SetCollisionEnabled` _mesh_2 "QueryAndPhysics")
      (`PrimitiveComponent.SetSimulatePhysics` _mesh_2 true)
      (`KismetSystemLibrary.Delay` 4.0)
      (`PrimitiveComponent.SetCollisionEnabled` (`Character.CapsuleComponent` (`self.FirstPersonCharacter`)) "QueryAndPhysics")
      (`PrimitiveComponent.SetCollisionObjectType` _mesh_3 "ECC_Pawn")
      (`PrimitiveComponent.SetCollisionEnabled` _mesh_3 "QueryOnly")
      (`PrimitiveComponent.SetSimulatePhysics` _mesh_3 false)
      (`SceneComponent.K2_SetWorldLocation` (`Character.CapsuleComponent` (`self.FirstPersonCharacter`)) (`SceneComponent.K2_GetComponentLocation` (`Character.Mesh` (`self.FirstPersonCharacter`))) false false)
      (`SceneComponent.K2_AttachToComponent` _mesh (`Character.CapsuleComponent` (`self.FirstPersonCharacter`)) "None" "SnapToTarget" "KeepRelative" "KeepRelative" true)
      (`SceneComponent.K2_SetRelativeLocationAndRotation` _mesh (0.0 0.0 -97.0) (struct :`Yaw` 270.0) false false)
      (`self.K2_SetActorLocationAndRotation` (`self.FirstPersonCharacter`) (`KismetMathLibrary.MakeVector` _returnvalue_x _returnvalue_y _returnvalue_z) (`self.K2_GetActorRotation` _playerstart) false true)
      (`self.EnableInput` (`self.FirstPersonCharacter`) (`GameplayStatics.GetPlayerController` 0)))))

(fn `UserConstructionScript`)